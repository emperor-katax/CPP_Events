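; BP_item_A is an item Blueprint that appears to be a test harness for calling functions and receiving events.
; BPEvent_01 passes a hard-coded name and ID to SetupValues, and BPEvent_02 calls Check01; neither function is defined in this graph.
; SetDetails, SkillSet and SkillControl only print "ktx"-tagged debug strings, with SetDetails including the received name and ID.
; BeginPlay, Tick, overlap and the construction script do nothing.
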(event `BPEvent_01`
  (`self.SetupValues` "Tokyo" 12))

(event `self.SetDetails`
  (params (Name :type String) (ID :type "Integer (by ref)"))
  (`KismetSystemLibrary.PrintString` (`KismetStringLibrary.Concat_StrStr` "ktx ---- " Name " + " (`KismetStringLibrary.Conv_IntToString` ID))))

(event `self.SkillSet`
  (`KismetSystemLibrary.PrintString` "ktx -- SkillSet event activated "))

(event `self.SkillControl`
  (`KismetSystemLibrary.PrintString` "ktx -- SkillControl event activated "))

(event `BPEvent_02`
  (`self.Check_01`))

(fn `UserConstructionScript`)